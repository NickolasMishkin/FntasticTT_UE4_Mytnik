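; Turtle actor that moves between its position and a target location passed to MoveTo, using a selectable movement mode.
; MoveTo stores both positions and calls Movement, which branches on InputMovementMode.
; Forward-Back mode runs a looping timer that alternates swept VInterpTo steps toward target and start, using accumulated delta-time counters.
; Forward mode takes only one step per call, and both Stand modes are empty stubs.
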(event Custom|MoveTo
  (params (DeltaLocation :type Vector))
  (Variables|Default|SetFinishPos DeltaLocation)
  (Variables|Default|SetStartPos (Transformation|GetActorLocation))
  (Variables|Default|SetCondition true)
  (CallFunction|Movement))

(event EventBeginPlay
  (Variables|Default|SetStartPos (Transformation|GetActorLocation)))

(fn ConstructionScript)

(fn MoveForward
  (Transformation|SetActorLocation (Math|Interpolation|VInterpTo (Transformation|GetActorLocation) (Variables|Default|GetFinishPos) (Utilities|Time|GetWorldDeltaSeconds) 1.0) true false))

(fn MoveBack
  (Transformation|SetActorLocation (Math|Interpolation|VInterpTo (Transformation|GetActorLocation) (Variables|Default|GetStartPos) (Utilities|Time|GetWorldDeltaSeconds) 1.0) true false))

(fn Stand)

(fn ResetCurrentTime
  (params (CurrentMoveForwardTime :type Float%20%28single-precision%29) (CurrentMoveBackTime :type Float%20%28single-precision%29))
  (Variables|Default|SetCurrentMoveForwardTime CurrentMoveForwardTime)
  (Variables|Default|SetCurrentMoveBackTime CurrentMoveBackTime))

(fn Movement
  (switch Utilities|FlowControl|Switch|SwitchonETurtleMovementMode (Variables|Default|GetInput%20Movement%20Mode)
    (:NewEnumerator0
      (CallFunction|MoveForward))
    (:NewEnumerator3
      (Utilities|Time|SetTimerbyFunctionName self "MoveForwardBack" 0.01 true))
    (:NewEnumerator4
      (CallFunction|MoveForwardStand))
    (:NewEnumerator5
      (CallFunction|MoveForwardBackStand))))

(fn MoveForwardBackStand)

(fn MoveForwardStand)

(fn MoveForwardBack
  (bind _returnvalue (Utilities|Time|GetWorldDeltaSeconds))
  (bind _output_get (Variables|Default|SetCurrentMoveForwardTime (+ (Variables|Default|GetCurrentMoveForwardTime) _returnvalue)))
  (if (>= _output_get (Variables|Default|GetMoveForwardTime))
    (Variables|Default|SetCurrentMoveBackTime (+ (Variables|Default|GetCurrentMoveBackTime) _returnvalue))
    (CallFunction|MoveBack)
    (if (>= (Variables|Default|GetCurrentMoveBackTime) (Variables|Default|GetMoveBackTime))
      (CallFunction|ResetCurrentTime 0.0 0.0))
    (else
      (CallFunction|MoveForward))))